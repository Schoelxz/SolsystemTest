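; Sphere2_Blueprint is a physics sphere that acts as a randomly sized body in an N-body gravity simulation.
; On BeginPlay it picks a random star mass, scales and weights the mesh from it, and gives it a random mass-scaled impulse.
; Each tick it applies the force vectors from its GravityUniversal component as amplified forces.
; On any hit it removes itself from GravityUniversal and is destroyed; older Sun-based gravity math remains unused.
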(event EventBeginPlay
  (bind _output_get (Variables|/Script/SolsystemFysik.GravityUniversal|Setstar_mass (Variables|Default|GetGravityUniversal) (Math|Random|RandomFloatinRange 1e+02 1e+07)))
  (Transformation|SetRelativeScale3D (Variables|Debug|GetStaticMeshComponent) (Math|Conversions|ToVector(Float) (/ _output_get 5e+04)))
  (Class|PrimitiveComponent|SetMassOverrideinKg (Variables|Debug|GetStaticMeshComponent) "None" _output_get true)
  (Physics|AddImpulse (Variables|Debug|GetStaticMeshComponent) (* (Math|Vector|MakeVector (Math|Random|RandomFloatinRange -1e+04 1e+04) (Math|Random|RandomFloatinRange -1e+04 1e+04) (Math|Random|RandomFloatinRange -1e+04 1e+04)) (/ _output_get 1e+01)) "None" false))

(event Collision|EventHit
  (params (MyComp :type Primitive%20Component%20Object%20Reference) (Other :type Actor%20Object%20Reference) (OtherComp :type Primitive%20Component%20Object%20Reference) (bSelfMoved :type Boolean) (HitLocation :type Vector :default "0, 0, 0") (HitNormal :type Vector :default "0, 0, 0") (NormalImpulse :type Vector :default "0, 0, 0") (Hit :type Hit%20Result%20Structure%20%28by%20ref%29))
  (Class|GravityUniversal|RemoveThis (Variables|Default|GetGravityUniversal))
  (Actor|DestroyActor))

(event EventTick
  (params (DeltaSeconds :type Float%20%28single-precision%29))
  (bind _returnvalue (Class|GravityUniversal|CalcResult (Variables|Default|GetGravityUniversal)))
  (for _array_element _returnvalue
    (Physics|AddForce (Variables|Debug|GetStaticMeshComponent) (* (* _array_element 5e+07) 5e+02) "None" false)))

(fn ConstructionScript)