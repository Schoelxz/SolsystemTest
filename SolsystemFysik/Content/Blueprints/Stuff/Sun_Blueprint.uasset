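; Sun actor that acts as a heavy physics-simulated star driven by a GravityUniversal component.
; On BeginPlay it sets a fixed star mass on both the component and the mesh, and optionally applies a random mass-scaled starting impulse.
; Each tick it applies every force vector returned by the component's CalcResult to the mesh, scaled by a large constant.
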(event EventBeginPlay
  (bind _output_get (Variables|/Script/SolsystemFysik.GravityUniversal|Setstar_mass (Variables|Default|GetGravityUniversal) 9e+07))
  (Class|PrimitiveComponent|SetMassOverrideinKg (Variables|Debug|GetStaticMeshComponent) "None" _output_get true)
  (if (Variables|Default|Getstart%20force%20impulse?)
    (Physics|AddImpulse (Variables|Debug|GetStaticMeshComponent) (* (Math|Vector|MakeVector (Math|Random|RandomFloatinRange -1e+04 1e+04) (Math|Random|RandomFloatinRange -1e+04 1e+04) (Math|Random|RandomFloatinRange -1e+04 1e+04)) (/ _output_get 1e+01)) "None" false)))

(event EventTick
  (params (DeltaSeconds :type Float%20%28single-precision%29))
  (bind _returnvalue (Class|GravityUniversal|CalcResult (Variables|Default|GetGravityUniversal)))
  (for _array_element _returnvalue
    (Physics|AddForce (Variables|Debug|GetStaticMeshComponent) (* _array_element 1e+07) "None" false)))

(fn ConstructionScript)