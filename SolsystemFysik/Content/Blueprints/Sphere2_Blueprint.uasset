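; Physics sphere, apparently a celestial body, that moves under simulated gravity.
; Each tick it gets an array of forces from GravityUniversal's CalcResult and applies each, scaled down by a constant, to its static mesh with AddForce.
; Disconnected leftover nodes hold an older hand-built Newtonian pull toward the sun, kept for reference and never executed.
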(event EventBeginPlay)

(event Collision|EventActorBeginOverlap
  (params (OtherActor :type Actor%20Object%20Reference)))

(event EventTick
  (params (DeltaSeconds :type Float%20%28single-precision%29))
  (bind _returnvalue (Class|GravityUniversal|CalcResult (Variables|Default|GetGravityUniversal)))
  (for _array_element _returnvalue
    (Physics|AddForce (Variables|Debug|GetStaticMeshComponent) (/ _array_element 8.0) "None" false)))

(fn ConstructionScript)