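; Sun actor Blueprint that acts as a physics-driven star under simulated gravity.
; On BeginPlay it passes the sun's mass to GravityUniversal, applies it as the mesh's mass override, and optionally adds a starting velocity-change impulse.
; Each tick it applies every vector returned by GravityUniversal's CalcResult to the mesh as a force, scaled by ForceMultiplier.
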(event EventBeginPlay
  (bind _output_get (Variables|/Script/SolsystemFysik.GravityUniversal|Setstar_mass (Variables|Default|GetGravityUniversal) (Variables|Default|GetSuns%20mass)))
  (Class|PrimitiveComponent|SetMassOverrideinKg (Variables|Debug|GetStaticMeshComponent) "None" _output_get true)
  (if (Variables|Default|Getstart%20force%20impulse?)
    (Physics|AddImpulse (Variables|Debug|GetStaticMeshComponent) (Math|Vector|MakeVector (Variables|Default|GetImpusle%20X) (Variables|Default|GetImpusle%20Y) (Variables|Default|GetImpulse%20Z)) "None" true)))

(event EventTick
  (params (DeltaSeconds :type Float%20%28single-precision%29))
  (bind _returnvalue (Class|GravityUniversal|CalcResult (Variables|Default|GetGravityUniversal)))
  (for _array_element _returnvalue
    (Physics|AddForce (Variables|Debug|GetStaticMeshComponent) (* _array_element (Variables|Default|GetForce%20Multiplier)) "None" false)))

(fn ConstructionScript)