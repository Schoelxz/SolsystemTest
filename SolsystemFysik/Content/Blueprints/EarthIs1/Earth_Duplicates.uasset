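; Earth_Duplicates is a planet actor that moves under simulated gravity through a GravityUniversal object and spins as it travels.
; On BeginPlay it copies its mass into GravityUniversal and the mesh's mass override, with an optional starting velocity impulse.
; Each tick it applies every force returned by CalcResult, scaled by a multiplier adjustable with debug-style number keys.
; Any hit removes it from GravityUniversal and destroys it.
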(event EventBeginPlay
  ;[1 1 1] Beginplay
  (bind _output_get (Variables|/Script/SolsystemFysik.GravityUniversal|Setstar_mass (Variables|Default|GetGravityUniversal) (Variables|Default|GetEarths%20Mass)))
  (Class|PrimitiveComponent|SetMassOverrideinKg (Variables|Debug|GetStaticMeshComponent) "None" _output_get true)
  (if (Variables|Default|Getstart%20force%20impulse?)
    (Physics|AddImpulse (Variables|Debug|GetStaticMeshComponent) (Math|Vector|MakeVector (Variables|Default|GetImpusle%20X) (Variables|Default|GetImpusle%20Y) (Variables|Default|GetImpulse%20Z)) "None" true)))

(event Collision|EventHit
  (params (MyComp :type Primitive%20Component%20Object%20Reference) (Other :type Actor%20Object%20Reference) (OtherComp :type Primitive%20Component%20Object%20Reference) (bSelfMoved :type Boolean) (HitLocation :type Vector :default "0, 0, 0") (HitNormal :type Vector :default "0, 0, 0") (NormalImpulse :type Vector :default "0, 0, 0") (Hit :type Hit%20Result%20Structure%20%28by%20ref%29))
  ;[1 1 1] Event Hit
  (Class|GravityUniversal|RemoveThis (Variables|Default|GetGravityUniversal))
  (Actor|DestroyActor))

(event EventTick
  (params (DeltaSeconds :type Float%20%28single-precision%29))
  (bind _staticmeshcomponent (Variables|Debug|GetStaticMeshComponent))
  ;[1 1 1] Event Tick
  (Utilities|FlowControl|Sequence
    (:then_0
      (bind _returnvalue (Class|GravityUniversal|CalcResult (Variables|Default|GetGravityUniversal)))
      (for _array_element _returnvalue
        (Physics|AddForce _staticmeshcomponent (* _array_element (Variables|Default|GetForce%20Multiplier)) "None" false)))
    (:then_1
      (Transformation|AddRelativeRotation _staticmeshcomponent (Math|Rotator|MakeRotator 0.0 (* DeltaSeconds 2.0) (* DeltaSeconds 3e+01)) false false))))

(event Input|KeyboardEvents|6
  (params (Key :type Key%20Structure))
  ;[1 1 1] Event Tick
  (:Pressed
    (bind _output_get (Variables|Default|SetForce%20Multiplier (+ (stale _output_get) 1e+03)))))

(event Input|KeyboardEvents|7
  (params (Key :type Key%20Structure))
  ;[1 1 1] Event Tick
  (:Pressed
    (bind _output_get (Variables|Default|SetForce%20Multiplier (- (stale _output_get) 1e+03)))))

(fn ConstructionScript)